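; BP_Isaac is the player character, adding hitscan shooting that also directs an allied AI.
; Shoot passes a camera-based trace along control rotation to the parent implementation, then emits a "Hearing" noise.
; Blocking hits on actors without the "Ally" tag receive damage and become the target in the blackboard of the BP_Ally found at BeginPlay.
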(event EventBeginPlay
  (bind _returnvalue (Actor|GetActorOfClass "/Game/Character/Ally/BP_Ally.BP_Ally_C"))
  (Variables|Default|SetAllyRef _returnvalue))

(event EventShoot
  (params (Start :type Vector :default "0, 0, 0") (End :type Vector :default "0, 0, 0"))
  (bind _returnvalue (Game|GetPlayerCameraManager 0))
  (bind _shoothit (Variables|Default|GetShootHit))
  (bind (_bblockinghit _binitialoverlap _time _distance _location _impactpoint _normal _impactnormal _physmat _hitactor) (Collision|BreakHitResult _shoothit))
  (bind _returnvalue_2 (Camera|GetCameraLocation _returnvalue))
  ;[1 1 1] Plyaer Shoot
  (|CallParentFunction _returnvalue_2 (+ _returnvalue_2 (* (Math|Vector|GetForwardVector (Pawn|GetControlRotation :!class /Script/Engine.Pawn)) (Variables|Default|GetShootRange))))
  (Class|Actor|MakeNoise 1.0 self (Transformation|GetActorLocation) 0.0 "Hearing")
  (if _bblockinghit
    (if (not (Actor|ActorHasTag _hitactor "Ally"))
      (Game|Damage|ApplyDamage _hitactor (Variables|Default|GetDamages) 0 0)
      (AI|Components|Blackboard|SetValueasObject (AI|GetBlackboard (AI|GetAIController (Variables|Default|GetAllyRef))) (Variables|Default|GetTargetRefKey) _hitactor))))

(fn ConstructionScript
  (|CallParentFunction))