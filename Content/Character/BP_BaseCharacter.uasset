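; BP_BaseCharacter is a base character Blueprint that provides health, death and a shooting trace.
; Health starts at MaxHealth on BeginPlay, drops with each AnyDamage event, and the actor is destroyed at zero or below.
; The Shoot event line-traces for Pawn objects between given points with timed debug drawing and stores the hit in ShootHit, without applying damage itself.
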(event Custom|Shoot
  (params (Start :type Vector) (End :type Vector))
  ;[1 1 1] Shoot
  (bind _outhit (Collision|LineTraceForObjects Start End (Utilities|Array|MakeArray "ObjectTypeQuery3") false 0 "ForDuration"))
  (Variables|Default|SetShootHit _outhit))

(event EventBeginPlay
  (Variables|Default|SetCurrentHealth (Variables|Default|GetMaxHealth)))

(event Game|Damage|EventAnyDamage
  (params (Damage :type Float%20%28single-precision%29) (DamageType :type Damage%20Type%20Object%20Reference) (InstigatedBy :type Controller%20Object%20Reference) (DamageCauser :type Actor%20Object%20Reference))
  ;[1 1 1] Apply Damage
  (bind _output_get (Variables|Default|SetCurrentHealth (- (Variables|Default|GetCurrentHealth) Damage)))
  (if (<= _output_get 0.0)
    (Actor|DestroyActor)))

(fn ConstructionScript)